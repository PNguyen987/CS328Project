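; Player pawn with free-flying camera movement and an in-world 3D cursor for clicking objects, plus a level prompt text.
; Holding right mouse hides the cursor and enables rotation of the camera sphere and camera-relative movement through FloatingPawnMovement, gated by CanMove.
; Otherwise mouse axes slide the MyMouse component within clamped bounds.
; Left click traces from the sphere through the cursor and calls Click on hit actors' Clickable components.
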(event `SetLevelText`
  (params (NewText :type Text))
  (set `self.LevelText` (`KismetTextLibrary.Conv_TextToString` NewText))
  (`TextRenderComponent.K2_SetText` (`self.Level`) NewText))

(event `self.ReceiveBeginPlay`
  (`self.EnableInput` self (`GameplayStatics.GetPlayerController` 0))
  (bind _output_get (set `self.LevelText` "Press Enter to Start Level"))
  (`TextRenderComponent.K2_SetText` (`self.Level`) (`KismetTextLibrary.Conv_StringToText` _output_get)))

(event `InputAction|LeftClick`
  (params (Key :type "Key Structure"))
  (bind _returnvalue (`SceneComponent.K2_GetComponentLocation` (`self.MyMouse`)))
  ;[1 1 1] Send the Click event to any clickable components in the Ray Trace
  (:`Pressed`
    (if (not (`self.HoldingRight`))
      (bind (_outhit _returnvalue_2) (`KismetSystemLibrary.LineTraceSingleForObjects` _returnvalue (+ _returnvalue (* (- _returnvalue (`SceneComponent.K2_GetComponentLocation` (`self.Sphere`))) 1000.0)) (`|MakeArray` "ObjectTypeQuery2" :!type "EObjectTypeQuery Enum") false (`|MakeArray` (`ChildActorComponent.ChildActor` (`self.MyMouse`)))))
      (if _returnvalue_2
        (bind (_bblockinghit _binitialoverlap _time _distance _location _impactpoint _normal _impactnormal _physmat _hitactor) (`GameplayStatics.BreakHitResult` _outhit))
        (`/Game/Blueprints/ActorComponents/Clickable.Click` (`self.K2_GetComponentsByClass` _hitactor "/Game/Blueprints/ActorComponents/Clickable.Clickable_C") _hitactor)))))

(event `InputAction|HoldRight`
  (params (Key :type "Key Structure"))
  ;[1 1 1] Can only move with the RMB pressed
  (:`Pressed`
    (set `self.HoldingRight` true)
    (set `self.MouseVisible` false)
    (`SceneComponent.SetVisibility` (`self.MyMouse`) (`self.MouseVisible`) false :!label _label))
  (:`Released`
    (set `self.HoldingRight` false)
    (set `self.MouseVisible` true)
    (goto _label)))

(event `InputAxis|MoveForward`
  (params (AxisValue :type "Float (single-precision)"))
  ;[1 1 1] Move forward and right
  (if (and (`self.HoldingRight`) (`self.CanMove`))
    (`self.AddMovementInput` (`SceneComponent.GetForwardVector` (`self.Camera`)) AxisValue true)))

(event `InputAxis|CameraUp`
  (params (AxisValue :type "Float (single-precision)"))
  (bind _sphere (`self.Sphere`))
  (bind _mymouse (`self.MyMouse`))
  ;[1 1 1] Camera Rotation Controller
  (if (`self.HoldingRight`)
    (`SceneComponent.K2_SetWorldRotation` _sphere (`KismetMathLibrary.MakeRotator` 0.0 (+ (* AxisValue (`self.CameraSpeed`)) (.pitch (`SceneComponent.K2_GetComponentRotation` _sphere))) (.yaw (`SceneComponent.K2_GetComponentRotation` _sphere))) false false)
    (else
      ;[1 1 1] Set position of mouse on screen and utilize the Keep Mouse Bounds Function
      (`SceneComponent.K2_AddRelativeLocation` _mymouse (`KismetMathLibrary.MakeVector` 0.0 0.0 (* AxisValue (`self.Mouse_Speed`))) false false)
      (`self.Keep Mouse Bounds` _mymouse :!label _label_2))))

(event `InputAxis|MoveRight`
  (params (AxisValue :type "Float (single-precision)"))
  ;[1 1 1] Move forward and right
  (if (and (`self.HoldingRight`) (`self.CanMove`))
    (`self.AddMovementInput` (`SceneComponent.GetRightVector` (`self.Camera`)) AxisValue true)))

(event `self.ReceiveTick`
  (params (DeltaSeconds :type "Float (single-precision)"))
  (bind _floatingpawnmovement (`self.FloatingPawnMovement`))
  ;[1 1 1] Adds Pending Input Vector to the actual movement component of the Pawn
  (if (`self.CanMove`)
    (bind _returnvalue (`PawnMovementComponent.ConsumeInputVector` _floatingpawnmovement))
    (`PawnMovementComponent.AddInputVector` _floatingpawnmovement _returnvalue false)
    (else
      (`MovementComponent.StopMovementImmediately` _floatingpawnmovement))))

(event `InputAxis|CameraRight`
  (params (AxisValue :type "Float (single-precision)"))
  (bind _sphere (`self.Sphere`))
  ;[1 1 1] Camera Rotation Controller
  (if (`self.HoldingRight`)
    (`SceneComponent.K2_SetWorldRotation` _sphere (`KismetMathLibrary.MakeRotator` 0.0 (.pitch (`SceneComponent.K2_GetComponentRotation` _sphere)) (+ (* (`self.CameraSpeed`) AxisValue) (.yaw (`SceneComponent.K2_GetComponentRotation` _sphere)))) false false)
    (else
      ;[1 1 1] Set position of mouse on screen and utilize the Keep Mouse Bounds Function
      (`SceneComponent.K2_AddRelativeLocation` (`self.MyMouse`) (`KismetMathLibrary.MakeVector` 0.0 (* AxisValue (`self.Mouse_Speed`))) false false)
      (goto _label_2))))

(fn `Keep Mouse Bounds`
  (params (Target :type "SceneComponent Object Reference"))
  (bind _z_max (`self.Z_max`))
  (bind _z_min (`self.Z_min`))
  (bind _y_max (`self.Y_max`))
  (bind _y_min (`self.Y_min`))
  (bind _location (.location (`SceneComponent.GetRelativeTransform` Target)))
  (bind _x (.x _location))
  (bind _y (.y _location))
  (bind _z (.z _location))
  (bind _x_2 (.x _location))
  (bind _y_2 (.y _location))
  (bind _z_2 (.z _location))
  ;[1 1 1] Set Z bounds
  (if (> _z _z_max)
    (`SceneComponent.K2_SetRelativeLocation` Target (`KismetMathLibrary.MakeVector` _x _y _z_max) false false))
  (if (< _z _z_min)
    (`SceneComponent.K2_SetRelativeLocation` Target (`KismetMathLibrary.MakeVector` _x _y _z_min) false false))
  ;[1 1 1] Set Y bounds
  (if (> _y_2 _y_max)
    (`SceneComponent.K2_SetRelativeLocation` Target (`KismetMathLibrary.MakeVector` _x_2 _y_max _z_2) false false))
  (if (< _y_2 _y_min)
    (`SceneComponent.K2_SetRelativeLocation` Target (`KismetMathLibrary.MakeVector` _x_2 _y_min _z_2) false false)))

(fn `UserConstructionScript`
  (bind _mymouse (`self.MyMouse`))
  (set `self.HoldingRight` false)
  (set `self.CameraSpeed` 2.0)
  (bind _output_get (set `self.MouseVisible` true))
  (`SceneComponent.SetVisibility` _mymouse _output_get false)
  (`SceneComponent.K2_SetRelativeLocation` _mymouse (200.0 0.0 0.0) false false)
  (set `self.Y_max` 199.0)
  (set `self.Y_min` -200.0)
  (set `self.Z_max` 100.0)
  (set `self.Z_min` -100.0)
  (set `self.Mouse_Speed` 4.0)
  (set `self.CanMove` true))