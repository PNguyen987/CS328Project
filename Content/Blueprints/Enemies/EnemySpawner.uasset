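; Enemy spawner actor that periodically spawns an AI enemy at its own location and rotation.
; Tick increments a counter each frame and, once it exceeds TOT, calls SpawnEnemy with EnemyCont1 and resets it, so the spawn rate depends on frame rate.
; SpawnEnemy uses SpawnAIFromClass with the EnemyBT behavior tree, then prints the blackboard's Goal vector as debug output.
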(event `self.ReceiveTick`
  (params (DeltaSeconds :type "Float (single-precision)"))
  (bind _iter (`self.Iter`))
  (if (> _iter (`self.TOT`))
    (`self.SpawnEnemy` "/Game/Blueprints/Enemies/Actors/EnemyCont1.EnemyCont1_C")
    (set `self.Iter` 0)
    (else
      (bind _result (`/Engine/EditorBlueprintResources/StandardMacros.IncrementInt` _iter)
        (:`  `
          (set `self.Iter` _result))))))

(event `SpawnEnemy`
  (params (ToSpawn :type "Pawn Class Reference"))
  (`AIBlueprintHelperLibrary.SpawnAIFromClass` ToSpawn "/Game/Blueprints/Enemies/AI/EnemyBT.EnemyBT" (.location (`self.GetTransform`)) (.rotation (`self.GetTransform`)) false null)
  (`KismetSystemLibrary.PrintString` (`KismetStringLibrary.Conv_VectorToString` (`BlackboardComponent.GetValueAsVector` (`AIBlueprintHelperLibrary.GetBlackboard` null) (`self.Goal`)))))

(fn `UserConstructionScript`)